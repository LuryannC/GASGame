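; GA_FireBolt is the Fire Bolt gameplay ability, which casts a projectile toward the point under the mouse.
; Target data sets the aim point, the avatar turns toward it through CombatInterface, then the ability commits, draws a debug sphere and plays the cast montage.
; A montage gameplay event triggers the projectile spawn, and montage completion ends the ability.
; A disconnected distance check is left unused.
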(event Ability|EventActivateAbility
  (bind _datahandle (|TargetDataUnderMouse)
    (:ValidDataDelegate
      (if (.bBlockingHit (Collision|BreakHitResult (Ability|TargetData|GetHitResultfromTargetData _datahandle)))
        (Variables|Default|SetProjectileTargetLocation (.ImpactPoint (Collision|BreakHitResult (Ability|TargetData|GetHitResultfromTargetData _datahandle))))
        (else
          (Variables|Default|SetProjectileTargetLocation (.TraceEnd (Collision|BreakHitResult (Ability|TargetData|GetHitResultfromTargetData _datahandle))))))
      (bind _ascombat_interface (Utilities|Casting|CastToCombatInterface (Ability|GetAvatarActorfromActorInfo))
        (:then
          (Class|CombatInterface|UpdateFacingTarget _ascombat_interface (Variables|Default|GetProjectileTargetLocation))
          (bind _returnvalue (Ability|CommitAbility))
          (if _returnvalue
            (Rendering|Debug|DrawDebugSphere (Variables|Default|GetProjectileTargetLocation) 5e+01 12 "(R=1.000000,G=0.000000,B=0.118320,A=1.000000)" 5.0)
            (|PlayMontageandWaitProxy "None" "/Game/Assets/Characters/Aura/Animations/Abilities/AM_Cast_FireBolt.AM_Cast_FireBolt" 1.0 "None" true 1.0 0.0 false
              (:then
                (Ability|Tasks|WaitGameplayEvent "(TagName=\"Event.Montage.FireBolt\")" 0
                  (:EventReceived
                    (Class|AuraProjectileSpell|SpawnProjectile (Variables|Default|GetProjectileTargetLocation)))))
              (:OnCompleted
                (Ability|EndAbility)))))
        (:CastFailed
          (Ability|EndAbility))))))